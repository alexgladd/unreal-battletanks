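; Player-controllable tank Blueprint that handles camera aiming, firing, driving and health bar setup.
; BeginPlay hands the turret and barrel to the aiming component, both tracks to the movement component, and itself to the HealthBar_BP widget.
; Aim axes rotate an azimuth gimbal for yaw and a spring arm for pitch, scaled by delta time.
; Fire and drive inputs forward to those components, with opposite directions sharing one function.
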(event EventBeginPlay
  (Class|TankAimingComponent|SetupAiming (Variables|Default|GetAimingComponent) (Variables|Default|GetTurret) (Variables|Default|GetBarrel))
  (Class|TankMovementComponent|Initialize (Variables|Default|GetMovementComponent) (Variables|Default|GetLeftTrack) (Variables|Default|GetRightTrack))
  (bind _ashealth_bar_bp (Utilities|Casting|CastToHealthBar_BP (UserInterface|GetUserWidgetObject (Variables|Default|GetWidget))))
  (Variables|/Game/Blueprints/HealthBar_BP.HealthBar_BP_C|SetTank _ashealth_bar_bp self))

(event Input|ActionEvents|InputActionFireGun
  (params (Key :type Key%20Structure :default "AnyKey"))
  ;[1 1 1] Firing
  (:Pressed
    (Class|TankAimingComponent|Fire (Variables|Default|GetAimingComponent))))

(event Input|AxisEvents|InputAxisMoveForward
  (params (AxisValue :type Float%20%28single-precision%29))
  ;[1 1 1] Movement
  (Class|TankMovementComponent|MoveForward (Variables|Default|GetMovementComponent) AxisValue))

(event Input|AxisEvents|InputAxisTurnRight
  (params (AxisValue :type Float%20%28single-precision%29))
  ;[1 1 1] Movement
  (Class|TankMovementComponent|TurnRight (Variables|Default|GetMovementComponent) AxisValue))

(event Input|AxisEvents|InputAxisMoveBackward
  (params (AxisValue :type Float%20%28single-precision%29))
  ;[1 1 1] Movement
  (Class|TankMovementComponent|MoveForward (Variables|Default|GetMovementComponent) AxisValue))

(event Input|AxisEvents|InputAxisTurnLeft
  (params (AxisValue :type Float%20%28single-precision%29))
  ;[1 1 1] Movement
  (Class|TankMovementComponent|TurnRight (Variables|Default|GetMovementComponent) AxisValue))

(event Input|AxisEvents|InputAxisAimAzimuth
  (params (AxisValue :type Float%20%28single-precision%29))
  ;[1 1 1] Azimuth Aiming
  (Transformation|AddLocalRotation (Variables|Default|GetAzimuthGimbal) (Math|Rotator|MakeRotator 0.0 0.0 (* AxisValue (Utilities|Time|GetWorldDeltaSeconds) 1e+02)) false false))

(event Input|AxisEvents|InputAxisAimElevation
  (params (AxisValue :type Float%20%28single-precision%29))
  ;[1 1 1] Elevation Aiming
  (Transformation|AddLocalRotation (Variables|Default|GetSpringArm) (Math|Rotator|MakeRotator 0.0 (* AxisValue (Utilities|Time|GetWorldDeltaSeconds) 1e+02) 0.0) false false))

(fn ConstructionScript)